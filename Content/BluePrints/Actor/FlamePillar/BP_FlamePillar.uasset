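; BP_FlamePillar is a flame pillar actor that flickers its point light to imitate fire.
; From BeginPlay, it randomly picks one of two intensity timelines, then picks again each time one finishes, looping indefinitely.
; Each timeline update feeds its track value to SetFlameIntencity, which multiplies it by BaseIntensity to set the PointLight's intensity.
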(event Custom|FlameIntencity_1
  (bind _intencitytrack (Timeline|FlameIntencityTimeLine_1 PlayFromStart)
    (:Update
      (CallFunction|SetFlameIntencity _intencitytrack))
    (:Finished
      (CallFunction|ChooseTimeLine))))

(event Custom|FlameIntencity_2
  (bind _intencitytrack (Timeline|FlameIntencityTimeLine_2 PlayFromStart)
    (:Update
      (CallFunction|SetFlameIntencity _intencitytrack))
    (:Finished
      (CallFunction|ChooseTimeLine))))

(event Custom|ChooseTimeLine
  (switch int (Math|Random|RandomIntegerinRange 0 1)
    (:Default
      (CallFunction|FlameIntencity2 :!label _label))
    (:0
      (CallFunction|FlameIntencity1))
    (:1
      (goto _label))))

(event EventBeginPlay
  (CallFunction|ChooseTimeLine))

(fn ConstructionScript)

(fn SetFlameIntencity
  (params (Intencity :type Float%20%28double-precision%29))
  (Rendering|Components|Light|SetIntensity (Variables|Default|GetPointLight) (* (Variables|Default|GetBaseIntensity) Intencity)))