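; Static mesh actor that can fade out and back in through a "Fade" material parameter.
; The construction script caches the original materials and creates dynamic instances, which FadeOut applies before playing a timeline that drives the parameter.
; Fadein reverses the timeline.
; At Fade 1 the original materials are restored; with BlockVisibility set, Visibility-channel collision blocks at 1 and is ignored at 0.
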(event EventBeginPlay)

(event EventFadein
  (bind _fade (Timeline|FadeTime Reverse)
    (:Update
      (for _array_element (Variables|Default|GetDynamicMaterialIntances)
        (Rendering|Material|SetScalarParameterValue _array_element "Fade" _fade :!class /Script/Engine.MaterialInstanceDynamic))
      (CallFunction|FadeFinished _fade))))

(event EventFadeOut
  (CallFunction|SetMaterialtoDynamicInstances)
  (bind _fade (Timeline|FadeTime Play)
    (:Update
      (for _array_element (Variables|Default|GetDynamicMaterialIntances)
        (Rendering|Material|SetScalarParameterValue _array_element "Fade" _fade :!class /Script/Engine.MaterialInstanceDynamic))
      (CallFunction|FadeFinished _fade))))

(fn ConstructionScript
  (Utilities|Array|Clear (Variables|Default|GetDynamicMaterialIntances))
  (bind _output_get (Variables|Default|SetOriginalMaterials (Rendering|Material|GetMaterials (Variables|Default|GetStaticMesh))))
  (for _array_element _output_get
    (bind _returnvalue (Rendering|Material|CreateDynamicMaterialInstance _array_element "None" "None" :!class /Script/Engine.KismetMaterialLibrary))
    (Utilities|Array|Add (Variables|Default|GetDynamicMaterialIntances) _returnvalue)))

(fn SetMaterialtoDynamicInstances
  (for (_array_element _array_index) (Variables|Default|GetDynamicMaterialIntances)
    (Rendering|Material|SetMaterial (Variables|Default|GetStaticMesh) _array_index _array_element)))

(fn ResetMaterials
  (for (_array_element _array_index) (Variables|Default|GetOriginalMaterials)
    (Rendering|Material|SetMaterial (Variables|Default|GetStaticMesh) _array_index _array_element)))

(fn FadeFinished
  (params (Fade :type Float%20%28double-precision%29))
  (if (>= Fade 1.0)
    (CallFunction|ResetMaterials)
    (if (Variables|Default|GetBlockVisibility)
      (Collision|SetCollisionResponsetoChannel (Variables|Default|GetStaticMesh) "ECC_Visibility" "ECR_Block"))
    (elif (<= Fade 0.0)
      (if (Variables|Default|GetBlockVisibility)
        (Collision|SetCollisionResponsetoChannel (Variables|Default|GetStaticMesh) "ECC_Visibility" "ECR_Ignore")))))