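; BP_FireBolt is the Fire Bolt projectile actor in the Phosphor fire abilities of the ability system.
; On BeginPlay it waits briefly before enabling query-only collision on its sphere component.
; Each Tick compares its location with the previous frame's to detect a stop, rather than using hit or overlap events.
; When movement falls to a minimum threshold, it spawns an impact sound and Niagara explosion, then destroys itself.
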(event EventBeginPlay
  (Utilities|FlowControl|Delay 0.1)
  (Collision|SetCollisionEnabled (Variables|Default|GetSphereComponent) "QueryOnly"))

(event Collision|EventActorBeginOverlap
  (params (OtherActor :type Actor%20Object%20Reference)))

(event EventTick
  (params (DeltaSeconds :type Float%20%28single-precision%29))
  (Variables|Default|SetLastFrameLocation (Variables|Default|GetThisLocation))
  (Variables|Default|SetThisLocation (Transformation|GetActorLocation))
  (if (<= (Math|Vector|VectorLength (- (Variables|Default|GetThisLocation) (Variables|Default|GetLastFrameLocation))) (Variables|Default|GetMinDistancePerFrame))
    (Audio|SpawnSoundatLocation "/Game/Assets/Sounds/Abilities/FireBolt/sfx_FireBolt_Impact.sfx_FireBolt_Impact" (Variables|Default|GetThisLocation) "0, 0, 0" 1.0 1.0 0.0 0 0)
    (Niagara|SpawnSystematLocation "/Game/Assets/Effects/Projectiles/FireExplosion/NS_FireExplosion.NS_FireExplosion" (Variables|Default|GetThisLocation))
    (Actor|DestroyActor)))

(fn ConstructionScript)