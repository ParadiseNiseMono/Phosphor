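; Arcane Shards gameplay ability that shows a magic circle, waits for a press, then erupts shards at the ground point under the mouse.
; A spawned BP_PointCollection supplies randomly rotated ground points, their count set by ability level up to a cap.
; A montage event commits the ability and starts a looping timer, spawning one shard cue per point.
; Each shard applies radial damage, knocking live targets outward, until the last ends the ability.
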(event Custom|SpawnShard
  (if (< (Variables|Default|GetCount) (Variables|Default|GetNum%20Points))
    (CallFunction|SetShardSpawnLocation)
    (CallFunction|StoreActorstoDamage)
    (for _array_element (Variables|Default|GetActorsToDamage)
      (CallFunction|ApplyRadialDamagetoActor _array_element))
    (Math|Integer|IncrementInt (Variables|Default|GetCount)
      (:%20%20
        (Class|GameplayAbility|ExecuteGameplayCuewithParams "(TagName=\"GameplayCue.ArcaneShards\")" (Ability|GameplayCue|MakeGameplayCueParameters :Location (Variables|Default|GetShardSpawnLocation)))))
    (else
      (Utilities|Time|ClearandInvalidateTimerbyHandle (Variables|Default|GetSpawnShardTimer))
      (Actor|DestroyActor (Variables|Default|GetPointCollection))
      (Ability|EndAbility))))

(event Ability|EventActivateAbility
  (bind _returnvalue (Class|GameplayAbility|CheckAbilityCost))
  (if _returnvalue
    (Utilities|FlowControl|Sequence
      (:then_0
        (Class|PlayerInterface|ShowMagicCircle(Message) (Ability|GetAvatarActorfromActorInfo) 0))
      (:then_1
        (Ability|Tasks|WaitInputPress false
          (:OnPress
            (Utilities|FlowControl|Sequence
              (:then_0
                (bind _datahandle (|TargetDataUnderMouse)
                  (:ValidData
                    (Variables|Default|SetImpact%20Point (.ImpactPoint (Collision|BreakHitResult (Ability|TargetData|GetHitResultfromTargetData _datahandle))))
                    (Variables|Default|SetNum%20Points (Math|Integer|Min(Integer) (Variables|Default|GetMaxNumShards) (Ability|GetAbilityLevel)))
                    (bind _returnvalue_2 (Game|SpawnActorfromClass "/Game/BluePrints/AbilitySystem/Phosphor/Abilities/Arcane/ArcaneShards/BP_PointCollection.BP_PointCollection_C" (Math|Transform|MakeTransform (Variables|Default|GetImpact%20Point) "0, 0, 0" "1.000000,1.000000,1.000000") "AlwaysSpawn" "MultiplyWithRoot" 0 0))
                    (Variables|Default|SetPointCollection _returnvalue_2)
                    (Variables|Default|SetGroundPoints (Class|PointCollection|GetGroundPoints _returnvalue_2 (Variables|Default|GetImpact%20Point) (Variables|Default|GetNum%20Points) (Math|Random|RandomFloatinRange 0.0 3.6e+02))))))
              (:then_1
                (Class|CombatInterface|UpdateFacingTarget(Message) (Ability|GetAvatarActorfromActorInfo) (Variables|Default|GetImpact%20Point))
                (|PlayMontageandWaitProxy "None" "/Game/Assets/Characters/Wolf/Animations/Ability/AM_ArcaneShards.AM_ArcaneShards" 1.0 "None" true 1.0 0.0 false
                  (:then
                    (Ability|Tasks|WaitGameplayEvent "(TagName=\"Event.Montage.ArcaneShards\")" 0 true
                      (:EventReceived
                        (bind _returnvalue_3 (Utilities|Time|SetTimerbyEvent (delegate Custom|SpawnShard) (Variables|Default|GetSpawnShardDeltaTime) true))
                        (Variables|Default|SetSpawnShardTimer _returnvalue_3)
                        (CallFunction|SpawnShard)
                        (Class|PlayerInterface|HideMagicCircle(Message) (Ability|GetAvatarActorfromActorInfo))
                        (Ability|CommitAbility)))))))))))))

(fn SetShardSpawnLocation
  (Variables|Default|SetShardSpawnLocation (Transformation|GetWorldLocation (Utilities|Array|Get(acopy) (Variables|Default|GetGroundPoints) (Variables|Default|GetCount)))))

(fn StoreActorstoDamage
  (bind _returnvalue (Ability|GetAvatarActorfromActorInfo))
  (bind _outoverlappingactors (Class|PhosphorAbilitySystemLibrary|GetLivePlayersWithinRadius _returnvalue (Utilities|Array|MakeArray _returnvalue) (Variables|Default|GetRadialDamageOuterRadius) (Variables|Default|GetShardSpawnLocation)))
  (Variables|Default|SetActorsToDamage _outoverlappingactors))

(fn ApplyRadialDamagetoActor
  (params (TargetActor :type Actor%20Object%20Reference))
  (bind _returnvalue (Transformation|GetActorLocation TargetActor))
  (bind _shardspawnlocation (Variables|Default|GetShardSpawnLocation))
  (bind _returnvalue_2 (- _returnvalue _shardspawnlocation))
  (Class|PhosphorAbilitySystemLibrary|ApplyDamageEffect (Class|PhosphorDamageGameplayAbility|MakeDamageEffectParamsfromDefaults TargetActor (Variables|Default|GetShardSpawnLocation) true _returnvalue_2 true _returnvalue_2 true 45.0)))