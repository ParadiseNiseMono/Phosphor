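; GA_MeleeAttack is a gameplay ability for a spear melee attack, with hit detection that only draws debug spheres and applies no damage yet.
; On activation it turns the avatar toward its combat target through CombatInterface and plays the attack montage.
; The montage's melee gameplay event triggers a radius query for live players around the combat socket, ignoring the avatar.
; Each player found is marked with a debug sphere, then the ability ends.
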(event Ability|EventActivateAbility
  (bind _returnvalue (Ability|GetAvatarActorfromActorInfo))
  (bind _returnvalue_2 (Ability|GetAvatarActorfromActorInfo))
  (bind _returnvalue_3 (Class|EnemyInterface|GetCombatTarget(Message) _returnvalue))
  (bind _ascombat_interface (Utilities|Casting|CastToCombatInterface _returnvalue))
  (Class|CombatInterface|UpdateFacingTarget _ascombat_interface (Transformation|GetActorLocation _returnvalue_3))
  (|PlayMontageandWaitProxy "None" "/Game/Assets/Enemies/Goblin/Animations/Spear/AM_Attack_Spear.AM_Attack_Spear" 1.0 "None" true 1.0 0.0 false
    (:then
      (Ability|Tasks|WaitGameplayEvent "(TagName=\"Event.Montage.Attack.Melee\")" 0
        (:EventReceived
          (bind _returnvalue_4 (Class|CombatInterface|GetCombatSocketLocation(Message) _returnvalue_2))
          (bind _outoverlappingactors (Class|PhosphorAbilitySystemLibrary|GetLivePlayersWithinRadius self (Utilities|Array|MakeArray _returnvalue_2) 45.0 _returnvalue_4))
          (for _array_element _outoverlappingactors
            (Rendering|Debug|DrawDebugSphere (Transformation|GetActorLocation _array_element) 2e+01 12 "(R=0.286142,G=1.000000,B=0.000000,A=1.000000)" 2.0))
          (Ability|EndAbility))))))

(event Ability|EventOnEndAbility
  (params (bWasCancelled :type Boolean)))